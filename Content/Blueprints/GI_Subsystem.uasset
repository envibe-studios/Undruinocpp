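; Game instance-side serial bridge for physical controller hardware, meant to turn device packets into player pawn messages for thruster repair, jack, weapons and reloading.
; Received bytes feed PacketParser, whose decoded packets were to be parsed by message type and forwarded with debug prints.
; Port opening, closing, receive binding and packet dispatch are all disconnected, so the connect, close and decode events do nothing.
; Repair Progress is parsed but never forwarded, even in that disconnected logic.
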(event `ConnectSerialPorts`)

(event `CloseSerialPorts`
  (params (EndPlayReason :type "EEndPlayReason Enum" :default "Destroyed")))

(event `OnByteReceived_Event`
  (params (Bytes :type "Array of Byte (by ref)"))
  (`PacketParserComponent.IngestBytes` (`self.PacketParser`) Bytes))

(event `self.PacketParser.OnPacketDecoded`
  (params (Packet :type "BenchPacket Structure")))