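; Serial bridge from ESP hardware controllers to the player pawn, opening a fixed COM port on BeginPlay and closing it on EndPlay.
; Received bytes bypass the port's parser and feed a PacketParser, whose decoded packets are switched by message type.
; Thruster repair, jack state, weapon and reload RFID tags, and per-side IMU aim and fire become pawn messages with debug prints.
; Repair Progress is parsed but unused.
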(event `self.ReceiveBeginPlay`
  (bind _serialport (`self.SerialPort`))
  (bind _returnvalue (`ArduinoBlueprintLibrary.CreateSerialPort`))
  (bind _output_get (set `self.SerialPort` _returnvalue))
  (bind _returnvalue_2 (`ArduinoSerialPort.Open` _output_get "COM8" 115200))
  (if _returnvalue_2
    (add `ArduinoSerialPort.OnByteReceived` _serialport (delegate `OnByteReceived_Event`))
    (`KismetSystemLibrary.PrintString` "Connected!")
    (add `ArduinoSerialPort.OnLineReceived` _serialport (delegate `OnLineReceived_Event`))
    (set `ArduinoSerialPort.bShowRawTapOnScreen` true _output_get)
    (set `ArduinoSerialPort.bDumpRawSerial` true _output_get)
    (set `ArduinoSerialPort.bBypassParser` true _output_get)
    (else
      (`KismetSystemLibrary.PrintString` "Error Connecting"))))

(event `OnByteReceived_Event`
  (params (Bytes :type "Array of Byte (by ref)"))
  (`PacketParserComponent.IngestBytes` (`self.PacketParser`) Bytes))

(event `self.ReceiveTick`
  (params (DeltaSeconds :type "Float (single-precision)")))

(event `OnLineReceived_Event`
  (params (Line :type String))
  (`KismetSystemLibrary.PrintString` Line))

(event `self.ReceiveEndPlay`
  (params (EndPlayReason :type "EEndPlayReason Enum" :default "Destroyed"))
  (`ArduinoSerialPort.Close` (`self.SerialPort`)))

(event `self.PacketParser.OnPacketDecoded`
  (params (Packet :type "BenchPacket Structure"))
  (bind (_ver _src _type _seq _len _payload) (break `BenchPacket` Packet))
  (bind (_outdata _returnvalue) (`EspPacketBP.ParseWeaponImuPayload` _payload))
  (bind (_outdata_2 _returnvalue_2) (`EspPacketBP.ParseJackStatePayload` _payload))
  (bind (_outdata_3 _returnvalue_3) (`EspPacketBP.ParseReloadTagPayload` _payload))
  (bind (_outdata_4 _returnvalue_4) (`EspPacketBP.ParseWeaponTagPayload` _payload))
  (bind (_outdata_5 _returnvalue_5) (`EspPacketBP.ParseWheelTurnPayload` _payload))
  (bind (_side _pitch _yaw _buttons) (break `WeaponImuData` _outdata))
  (bind (_side_2 _uid) (break `WeaponTagData` _outdata_4))
  (bind _uid_2 (break `ReloadTagData` _outdata_3))
  (bind _returnvalue_6 (`KismetMathLibrary.Conv_ByteToInt` (`.State` (break `JackStateData` _outdata_2))))
  (bind _returnvalue_7 (`KismetMathLibrary.Conv_ByteToInt` (`.WheelIndex` (break `WheelTurnData` _outdata_5))))
  (bind _returnvalue_8 (== _side_2 0))
  (bind _returnvalue_9 (== _buttons 1))
  (bind _returnvalue_10 (== _side 0))
  (bind _returnvalue_11 (`KismetMathLibrary.MakeRotator` 0.0 (`KismetMathLibrary.Conv_IntToDouble` _pitch) (`KismetMathLibrary.Conv_IntToDouble` _yaw)))
  (switch `EEspMsgType` (`EspPacketBP.ByteToMsgType` _type)
    (:`WheelTurn`
      (if _returnvalue_5
        (message `/Game/Blueprints/BPI_ESPComms.ThrusterRepairPing` (`GameplayStatics.GetPlayerPawn` 0) _returnvalue_7)
        (`KismetSystemLibrary.PrintString` (`KismetStringLibrary.Concat_StrStr` "Thruster Repair, Thruster Index: " (`KismetStringLibrary.Conv_IntToString` _returnvalue_7)))))
    (:`RepairProgress`
      (if (`.ReturnValue` (`EspPacketBP.ParseRepairProgressPayload` _payload))
        _))
    (:`JackState`
      (if _returnvalue_2
        (message `/Game/Blueprints/BPI_ESPComms.JackState` (`GameplayStatics.GetPlayerPawn` 0) _returnvalue_6)
        (`KismetSystemLibrary.PrintString` (`KismetStringLibrary.Concat_StrStr` "Jack's State: " (`KismetStringLibrary.Conv_IntToString` _returnvalue_6)))))
    (:`WeaponTag`
      (if _returnvalue_4
        (message `/Game/Blueprints/BPI_ESPComms.WeaponTag` (`GameplayStatics.GetPlayerPawn` 0) _uid _returnvalue_8)
        (`KismetSystemLibrary.PrintString` (`KismetStringLibrary.Concat_StrStr` "Weapon Tag. PORT? " (`KismetStringLibrary.Conv_BoolToString` _returnvalue_8) " \nRFID: " (`KismetStringLibrary.Conv_Int64ToString` _uid)))))
    (:`ReloadTag`
      (if _returnvalue_3
        (message `/Game/Blueprints/BPI_ESPComms.ReloadTag` (`GameplayStatics.GetPlayerPawn` 0) _uid_2)
        (`KismetSystemLibrary.PrintString` (`KismetStringLibrary.Concat_StrStr` "Reload Tag RFID: " (`KismetStringLibrary.Conv_Int64ToString` _uid_2)))))
    (:`WeaponImu`
      (if _returnvalue
        (message `/Game/Blueprints/BPI_ESPComms.WeaponAim` (`GameplayStatics.GetPlayerPawn` 0) _returnvalue_11 _returnvalue_10)
        (message `/Game/Blueprints/BPI_ESPComms.WeaponFire` (`GameplayStatics.GetPlayerPawn` 0) _returnvalue_9 _returnvalue_10)
        (`KismetSystemLibrary.PrintString` (`KismetStringLibrary.Concat_StrStr` "Weapon Info PORT? " (`KismetStringLibrary.Conv_BoolToString` _returnvalue_10) " \nFiring? " (`KismetStringLibrary.Conv_BoolToString` _returnvalue_9) " \nRotator: " (`KismetStringLibrary.Conv_RotatorToString` _returnvalue_11)))))))

(fn `UserConstructionScript`)