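; GameMode Blueprint that opens and manages serial port connections for a list of ships.
; On BeginPlay with authority, it registers each ship's ID and port name with the AndySerialSubsystem at a fixed baud rate, printing the result to screen.
; It then starts all ports through the subsystem and stops them all on EndPlay.
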(event `self.ReceiveBeginPlay`
  (if (`self.HasAuthority`)
    (for _array_element (`self.Ships`)
      (bind (_shipid _portname) (break `/Game/Blueprints/PortRecord` _array_element))
      (bind _returnvalue (`AndySerialSubsystem.AddPort` (subsystem `AndySerialSubsystem`) _shipid _portname 115200))
      (if _returnvalue
        (bind _returnvalue_2 (`KismetStringLibrary.Conv_NameToString` _shipid))
        (`KismetSystemLibrary.PrintString` (`KismetStringLibrary.Concat_StrStr` _returnvalue_2 " Connected!"))
        (else
          (`KismetSystemLibrary.PrintString` (`KismetStringLibrary.Concat_StrStr` _returnvalue_2 "Had an error Connecting")))))
    (`AndySerialSubsystem.StartAll` (subsystem `AndySerialSubsystem`))))

(event `self.ReceiveEndPlay`
  (params (EndPlayReason :type "EEndPlayReason Enum" :default "Destroyed"))
  (if (`self.HasAuthority`)
    (`AndySerialSubsystem.StopAll` (subsystem `AndySerialSubsystem`))))

(fn `UserConstructionScript`)