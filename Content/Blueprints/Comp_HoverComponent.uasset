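; Hover thruster component that pushes a physics-simulated mesh away from surfaces below it, with the mesh supplied through InitComponents.
; Each tick it box-traces along its negative up vector for world static and dynamic objects, with optional debug drawing.
; On a hit, a damped spring calculation turns compression and its rate of change into an upward force applied at the component's location.
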(event `InitComponents`
  (params (MeshComponent :type "StaticMeshComponent Object Reference"))
  (bind _output_get (set `self.ParentComponent` MeshComponent))
  (`PrimitiveComponent.SetSimulatePhysics` _output_get true))

(event `self.ReceiveTick`
  (params (DeltaSeconds :type "Float (single-precision)"))
  (`self.ThrusterPhysics`))

(fn `ThrusterPhysics`
  (bind _returnvalue (`self.K2_GetComponentLocation`))
  (bind _hoverheight (`self.HoverHeight`))
  (bind (_outhit _returnvalue_2) (`KismetSystemLibrary.BoxTraceSingleForObjects` _returnvalue (- _returnvalue (* (`self.GetUpVector`) (`self.HoverHeight`))) (60.0 130.0 45.0) (struct) (`|MakeArray` "ObjectTypeQuery1" "ObjectTypeQuery2" :!type "EObjectTypeQuery Enum") false (`|MakeArray` (`self.GetOwner`)) (select `bool` (`self.debugRay`) :`true` "ForOneFrame" :!type "EDrawDebugTrace Enum")))
  (if _returnvalue_2
    (bind _returnvalue_3 (/ (- _hoverheight (`.Distance` (`GameplayStatics.BreakHitResult` _outhit))) _hoverheight))
    (set `self.HoverForce` (+ (* (/ (- _returnvalue_3 (`self.PreviousCompression`)) (`GameplayStatics.GetWorldDeltaSeconds`)) (`self.Damping`)) (* _returnvalue_3 (`self.Stiffness`))))
    (set `self.PreviousCompression` _returnvalue_3)
    (`PrimitiveComponent.AddForceAtLocation` (`self.ParentComponent`) (* (`self.GetUpVector`) (`self.HoverForce`)) (`self.K2_GetComponentLocation`) "None")
    (return)))